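; BP_Switch is an interactable switch that triggers a random item spawn when used.
; On interaction it calls its OnSwitchActivate event dispatcher, to which it binds its own handler at BeginPlay.
; The handler calls RandomSpawn on the referenced RandomItemSpawner if that reference is valid.
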(event `self.ReceiveBeginPlay`
  (`parent.ReceiveBeginPlay`)
  (add `self.OnSwitchActivate` (`|CreateDelegate` :!event `OnSwitchActivate_Event`)))

(event `self.OnInteract`
  (params (InteractingActor :type "Actor Object Reference"))
  (`self.OnSwitchActivate`))

(event `OnSwitchActivate_Event`
  (bind _random_item_spawner (`self.Random Item Spawner`))
  (`/Engine/EditorBlueprintResources/StandardMacros.IsValid` _random_item_spawner
    (:`Is Valid`
      (`/Game/CreativeTask/Placeables/BP_RandomItemSpawner.RandomSpawn` _random_item_spawner))))

(fn `UserConstructionScript`
  (`parent.UserConstructionScript`))