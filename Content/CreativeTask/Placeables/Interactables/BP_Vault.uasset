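; BP_Vault is an interactable vault that opens once and spawns a configurable item.
; The first OnInteract passes a DoOnce, then calls OnOpen, which spawns the item class at the Scene component's world transform, ignoring collision.
; It then plays a timeline that rotates the Head component's pitch toward a Rotation value.
; The lerp starts from Head's current roll rather than its pitch, re-read on each update.
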(event `self.OnInteract`
  (params (InteractingActor :type "Actor Object Reference"))
  (bind _relativerotation_roll (`KismetMathLibrary.BreakRotator` (`SceneComponent.RelativeRotation` (`self.Head`))))
  (`/Engine/EditorBlueprintResources/StandardMacros.DoOnce` false
    (:`Completed`
      (`self.On Open`)
      (bind (_direction _speed) (`Timeline|Timeline` :!via `PlayFromStart`)
        (:`Update`
          (`SceneComponent.K2_SetRelativeRotation` (`self.Head`) (`KismetMathLibrary.MakeRotator` 0.0 (`KismetMathLibrary.Lerp` _relativerotation_roll (`self.Rotation`) _speed)) false false))))))

(event `On Open`
  (`|SpawnActorFromClass` (`self.Item Classs To Spawn`) (`SceneComponent.K2_GetComponentToWorld` (`self.Scene`)) "AlwaysSpawn" "MultiplyWithRoot" null null))

(fn `UserConstructionScript`
  (`parent.UserConstructionScript`))