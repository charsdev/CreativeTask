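; Sliding door Blueprint that moves its Door component vertically between two preset heights.
; Each Open call alternates the target height through a FlipFlop and restarts a shared Timeline, so the same event raises and lowers the door.
; Timeline updates set relative Z with a sinusoidal ease from the door's current height toward the target, using the Speed track divided by Delay as alpha.
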(event `self.ReceiveBeginPlay`
  (`parent.ReceiveBeginPlay`))

(event `Open`
  (bind (_relativelocation_x _relativelocation_y _relativelocation_z) (`KismetMathLibrary.BreakVector` (`SceneComponent.RelativeLocation` (`self.Door`))))
  (`/Engine/EditorBlueprintResources/StandardMacros.FlipFlop`
    (:`A`
      (set `self.Location` 285.0)
      (bind (_direction _speed) (`Timeline|Timeline` :!via `PlayFromStart` :!label _label)
        (:`Update`
          (`SceneComponent.K2_SetRelativeLocation` (`self.Door`) (`KismetMathLibrary.MakeVector` 0.0 0.0 (`|EaseFunction` "SinusoidalInOut" (/ _speed (`self.Delay`)) _relativelocation_z (`self.Location`))) false false))))
    (:`B`
      (set `self.Location` 85.0)
      (goto _label :!via `PlayFromStart`))))

(fn `UserConstructionScript`
  (`parent.UserConstructionScript`))