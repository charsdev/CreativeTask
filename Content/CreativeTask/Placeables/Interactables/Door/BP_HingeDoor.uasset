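; BP_HingeDoor is an interactable hinged door that swings open and closed.
; Each OnInteract alternates the target yaw between FinalRotation and zero through a FlipFlop, then plays a shared Timeline from the start.
; Timeline updates divide the Speed track by Delay to drive a sinusoidal in-out ease of the door's relative yaw, blending from its current yaw each update toward the target.
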(event `self.ReceiveBeginPlay`
  (`parent.ReceiveBeginPlay`))

(event `self.OnInteract`
  (params (InteractingActor :type "Actor Object Reference"))
  (bind (_relativerotation_roll _relativerotation_pitch _relativerotation_yaw) (`KismetMathLibrary.BreakRotator` (`SceneComponent.RelativeRotation` (`self.Door`))))
  (`/Engine/EditorBlueprintResources/StandardMacros.FlipFlop`
    (:`A`
      (set `self.Rotation` (`self.FinalRotation`))
      (bind (_direction _speed) (`Timeline|Timeline` :!via `PlayFromStart` :!label _label)
        (:`Update`
          (`SceneComponent.K2_SetRelativeRotation` (`self.Door`) (`KismetMathLibrary.MakeRotator` 0.0 0.0 (`|EaseFunction` "SinusoidalInOut" (/ _speed (`self.Delay`)) _relativerotation_yaw (`self.Rotation`))) false false))))
    (:`B`
      (set `self.Rotation` 0.0)
      (goto _label :!via `PlayFromStart`))))

(fn `UserConstructionScript`
  (`parent.UserConstructionScript`))