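; Automatic sliding double door that opens when a Character enters its Box trigger and reverses when one leaves.
; Overlap begin plays a Timeline from the start; overlap end negates the offset and reverses it from the end.
; Each update moves both leaves in opposite directions with a sinusoidal ease from their current relative locations, so movement accumulates.
; The left leaf's initial location is saved at BeginPlay but never read.
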(event `self.ReceiveBeginPlay`
  (`parent.ReceiveBeginPlay`)
  (set `self.Initial Location` (`SceneComponent.RelativeLocation` (`self.DoorLeft`))))

(event `self.Box.OnComponentBeginOverlap`
  (params (OverlappedComponent :type "PrimitiveComponent Object Reference") (OtherActor :type "Actor Object Reference") (OtherComp :type "PrimitiveComponent Object Reference") (OtherBodyIndex :type Integer) (bFromSweep :type Boolean) (SweepResult :type "HitResult Structure (by ref)"))
  (cast `Character` OtherActor)
  (set `self.Location` (`self.Target Location`))
  (bind (_direction _newtrack_0) (`Timeline|Timeline` :!via `PlayFromStart` :!label _label)
    (:`Update`
      (bind _returnvalue (/ _newtrack_0 (`self.Delay`)))
      (`SceneComponent.K2_SetRelativeLocation` (`self.DoorLeft`) (`|EaseFunction` "SinusoidalInOut" _returnvalue (`SceneComponent.RelativeLocation` (`self.DoorLeft`)) (+ (`SceneComponent.RelativeLocation` (`self.DoorLeft`)) (`self.Location`))) false false)
      (`SceneComponent.K2_SetRelativeLocation` (`self.DoorRIght`) (`|EaseFunction` "SinusoidalInOut" _returnvalue (`SceneComponent.RelativeLocation` (`self.DoorRIght`)) (+ (`SceneComponent.RelativeLocation` (`self.DoorRIght`)) (* (`self.Location`) -1.0))) false false))))

(event `self.Box.OnComponentEndOverlap`
  (params (OverlappedComponent :type "PrimitiveComponent Object Reference") (OtherActor :type "Actor Object Reference") (OtherComp :type "PrimitiveComponent Object Reference") (OtherBodyIndex :type Integer))
  (cast `Character` OtherActor)
  (set `self.Location` (* (`self.Target Location`) -1.0))
  (goto _label :!via `ReverseFromEnd`))

(fn `UserConstructionScript`
  (`parent.UserConstructionScript`))