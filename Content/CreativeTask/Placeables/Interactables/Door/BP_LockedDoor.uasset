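; BP_LockedDoor is an interactable hinged door that can be locked behind required inventory items.
; On interact, a Door.IsLocked gameplay tag triggers an inventory check; success removes the tag, consumes the items and toggles the door.
; Failure shows the required items through the announcer subsystem.
; A FlipFlop alternates the target yaw between open and closed, and a timeline eases the door toward it.
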(event `self.ReceiveBeginPlay`
  (`parent.ReceiveBeginPlay`))

(event `self.OnInteract`
  (params (InteractingActor :type "Actor Object Reference"))
  (bind _returnvalue (`self.GetComponentByClass` InteractingActor "/Script/CreativeTask.Inventory"))
  (if (`BlueprintGameplayTagLibrary.HasTag` (`self.TagsContainer`) (struct :`TagName` "Door.IsLocked") true)
    (bind _hasrequireditems (`self.CheckHasRequiredItems` _returnvalue))
    (if _hasrequireditems
      (`BlueprintGameplayTagLibrary.RemoveGameplayTag` (`self.TagsContainer`) (struct :`TagName` "Door.IsLocked"))
      (for _array_element (`self.RequiredItems`)
        (bind (_item _quantity) (break `/Game/CreativeTask/Structs/F_RequiredItem` _array_element))
        (`Inventory.TryRemoveFromSlotItem` _returnvalue _item _quantity))
      (`self.ToogleDoor`)
      (else
        (`self.ShowRequiredItems`)))
    (else
      (`self.ToogleDoor`))))

(event `ToogleDoor`
  (bind (_relativerotation_roll _relativerotation_pitch _relativerotation_yaw) (`KismetMathLibrary.BreakRotator` (`SceneComponent.RelativeRotation` (`self.Door`))))
  (`/Engine/EditorBlueprintResources/StandardMacros.FlipFlop`
    (:`A`
      (set `self.Rotation` 110.0)
      (bind (_direction _speed) (`Timeline|Timeline` :!via `PlayFromStart` :!label _label)
        (:`Update`
          (`SceneComponent.K2_SetRelativeRotation` (`self.Door`) (`KismetMathLibrary.MakeRotator` 0.0 0.0 (`|EaseFunction` "SinusoidalInOut" (/ _speed (`self.Delay`)) _relativerotation_yaw (`self.Rotation`))) false false))))
    (:`B`
      (set `self.Rotation` 0.0)
      (goto _label :!via `PlayFromStart`))))

(fn `CheckHasRequiredItems`
  (params (InventoryFromInteractingActor :type "Inventory Object Reference"))
  (returns (HasRequiredItems :type Boolean))
  (locals (RequiredItemNames :type "Array of Name"))
  (for _array_element (`self.RequiredItems`)
    (bind (_item _quantity) (break `/Game/CreativeTask/Structs/F_RequiredItem` _array_element))
    (bind _returnvalue (`Inventory.HasItem` (`local.InventoryFromInteractingActor`) _item _quantity))
    (if (not _returnvalue)
      (return false)))
  (return true))

(fn `ShowRequiredItems`
  (locals (Result :type String))
  (set `local.Result` "<Danger>Requires: </>")
  (for _array_element (`self.RequiredItems`)
    (bind (_item _quantity) (break `/Game/CreativeTask/Structs/F_RequiredItem` _array_element))
    (set `local.Result` (`KismetStringLibrary.Concat_StrStr` (`local.Result`) " \n" (`KismetStringLibrary.Conv_NameToString` (`ItemData.ItemName` _item)) " <Warning>" " x" (`KismetStringLibrary.Conv_IntToString` _quantity) "</>")))
  (`AnnouncerSubsystem.ShowMessage` (subsystem `AnnouncerSubsystem`) (`KismetTextLibrary.Conv_StringToText` (`local.Result`)) 3.0))

(fn `UserConstructionScript`
  (`parent.UserConstructionScript`))