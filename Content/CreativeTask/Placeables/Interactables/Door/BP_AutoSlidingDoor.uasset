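; BP_AutoSlidingDoor is a door actor that slides vertically when a Character enters its Box trigger and returns when one leaves.
; Overlap events set the destination to either TargetZLocation or the Z recorded at BeginPlay, then restart a shared Timeline.
; Each update eases the door's current relative Z toward that destination with SinusoidalInOut, using the timeline's Speed track divided by Delay as alpha.
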(event `self.ReceiveBeginPlay`
  (`parent.ReceiveBeginPlay`)
  (set `self.InitialZLocation` (.z (`SceneComponent.RelativeLocation` (`self.Door`)))))

(event `self.Box.OnComponentBeginOverlap`
  (params (OverlappedComponent :type "PrimitiveComponent Object Reference") (OtherActor :type "Actor Object Reference") (OtherComp :type "PrimitiveComponent Object Reference") (OtherBodyIndex :type Integer) (bFromSweep :type Boolean) (SweepResult :type "HitResult Structure (by ref)"))
  (bind (_relativelocation_x _relativelocation_y _relativelocation_z) (`KismetMathLibrary.BreakVector` (`SceneComponent.RelativeLocation` (`self.Door`))))
  (cast `Character` OtherActor)
  (set `self.Location` (`self.TargetZLocation`))
  (bind (_direction _speed) (`Timeline|Timeline` :!via `PlayFromStart` :!label _label)
    (:`Update`
      (`SceneComponent.K2_SetRelativeLocation` (`self.Door`) (`KismetMathLibrary.MakeVector` 0.0 0.0 (`|EaseFunction` "SinusoidalInOut" (/ _speed (`self.Delay`)) _relativelocation_z (`self.Location`))) false false))))

(event `self.Box.OnComponentEndOverlap`
  (params (OverlappedComponent :type "PrimitiveComponent Object Reference") (OtherActor :type "Actor Object Reference") (OtherComp :type "PrimitiveComponent Object Reference") (OtherBodyIndex :type Integer))
  (cast `Character` OtherActor)
  (set `self.Location` (`self.InitialZLocation`))
  (goto _label :!via `PlayFromStart`))

(fn `UserConstructionScript`
  (`parent.UserConstructionScript`))