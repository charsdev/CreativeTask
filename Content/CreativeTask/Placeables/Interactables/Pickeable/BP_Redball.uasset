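; BP_Redball is a pooled red ball actor, filed under the creative task's pickable interactable placeables.
; It toggles physics on its SkeletalMesh with the pool lifecycle: activation enables simulation and gravity, and return to pool runs the parent logic, then disables both.
; Activation makes no parent call, the construction script only calls its parent, and the BeginPlay, overlap and Tick events are disabled stubs.
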(event `self.ReturnToPool`
  (bind _skeletalmesh (`self.SkeletalMesh`))
  (`parent.ReturnToPool`)
  (`PrimitiveComponent.SetEnableGravity` _skeletalmesh false)
  (`PrimitiveComponent.SetSimulatePhysics` _skeletalmesh false))

(event `self.OnPoolActivated`
  (bind _skeletalmesh (`self.SkeletalMesh`))
  (`PrimitiveComponent.SetSimulatePhysics` _skeletalmesh true)
  (`PrimitiveComponent.SetEnableGravity` _skeletalmesh true))

(fn `UserConstructionScript`
  (`parent.UserConstructionScript`))