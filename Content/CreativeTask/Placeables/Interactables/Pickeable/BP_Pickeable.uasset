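; BP_Pickeable is an interactable item pickup that a player collects into their inventory.
; On BeginPlay it registers itself with the object pool subsystem.
; When BP_Player interacts, it async-loads its item data primary asset and tries to add one to the player's Inventory component.
; If the add succeeds, the pickup returns itself to the pool.
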(event `self.ReceiveBeginPlay`
  (`parent.ReceiveBeginPlay`)
  (`ObjectPoolSubsystem.AddToPool` (subsystem `ObjectPoolSubsystem`) self))

(event `self.ReturnToPool`
  (`ObjectPoolSubsystem.ReturnToPool` (subsystem `ObjectPoolSubsystem`) self))

(event `self.OnInteract`
  (params (InteractingActor :type "Actor Object Reference"))
  (bind _asbp_player (cast `/Game/CreativeTask/Characters/Mannequin/BP_Player` InteractingActor))
  (bind _loaded (`AsyncActionLoadPrimaryAsset.AsyncLoadPrimaryAsset` (`self.ItemDataInventory`))
    (:`then`
      (bind _asitem_data (cast `ItemData` _loaded))
      (bind _returnvalue (`self.GetComponentByClass` _asbp_player "/Script/CreativeTask.Inventory"))
      (`/Engine/EditorBlueprintResources/StandardMacros.IsValid` _returnvalue
        (:`Is Valid`
          (bind (_outslotindex _outquantity _returnvalue_2) (`Inventory.TryAddItemToSlot` _returnvalue _asitem_data 1))
          (if _returnvalue_2
            (`self.ReturnToPool`)))))))

(fn `UserConstructionScript`
  (`parent.UserConstructionScript`))