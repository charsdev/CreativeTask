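; BP_DirectionalLightPhong is a placeable light direction source for Phong shading.
; It writes its negated forward vector to the LightDirection parameter of the MPC_Phong material parameter collection, both in the construction script and every tick.
; On BeginPlay it also stores its offset from the player pawn in InitialOffset, which none of its graphs read.
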(event `self.ReceiveBeginPlay`
  (set `self.Initial offset` (- (`self.K2_GetActorLocation`) (`self.K2_GetActorLocation` (`GameplayStatics.GetPlayerPawn` 0)))))

(event `self.ReceiveTick`
  (params (DeltaSeconds :type "Float (single-precision)"))
  (`self.UpdateLightDirection`))

(fn `UpdateLightDirection`
  (`KismetMaterialLibrary.SetVectorParameterValue` "/Game/CreativeTask/Art/Materials/Phong/MPC_Phong.MPC_Phong" "LightDirection" (`KismetMathLibrary.Conv_VectorToLinearColor` (* (`self.GetActorForwardVector`) -1.0))))

(fn `UserConstructionScript`
  (`self.UpdateLightDirection`))