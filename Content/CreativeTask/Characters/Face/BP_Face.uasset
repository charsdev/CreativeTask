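; BP_Face is a talking face character that dissolves in when spawned and dissolves out once it stops talking.
; BeginPlay puts a dynamic MI_Dissolve material on the skeletal mesh and runs a reversed timeline to animate DissolveAmount.
; Talk and FinishTalk ramp TalkSpeed on ABP_Face up or down through per-tick interpolation loops.
; After FinishTalk winds down, it waits briefly, plays the dissolve forward, then fires OnFinishTalk.
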(event `self.ReceiveBeginPlay`
  (bind _asabp_face (cast `/Game/CreativeTask/Characters/Face/ABP_Face` (`SkeletalMeshComponent.GetAnimInstance` (`self.SkeletalMesh`))))
  (set `self. ABP Face Mask` _asabp_face)
  (bind _returnvalue (`KismetMaterialLibrary.CreateDynamicMaterialInstance` "/Game/CreativeTask/Art/Materials/MI_Dissolve.MI_Dissolve"))
  (bind _output_get (set `self.DMI` _returnvalue))
  (`PrimitiveComponent.SetMaterial` (`self.SkeletalMesh`) 0 _output_get)
  (bind (_direction _dissolvetrack) (`Timeline|Timeline_0` :!via `ReverseFromEnd`)
    (:`Update`
      (`MaterialInstanceDynamic.SetScalarParameterValue` (`self.DMI`) "DissolveAmount" _dissolvetrack))))

(event `Talk`
  (bind __abp_face_mask (`self. ABP Face Mask`))
  (bind _talkspeed (`/Game/CreativeTask/Characters/Face/ABP_Face.TalkSpeed` __abp_face_mask))
  (if (< _talkspeed 1.0) :!label _label
    (`KismetSystemLibrary.DelayUntilNextTick`)
    (set `/Game/CreativeTask/Characters/Face/ABP_Face.TalkSpeed` (`KismetMathLibrary.FInterpTo_Constant` _talkspeed 1.0 (`GameplayStatics.GetWorldDeltaSeconds`) 1.0) __abp_face_mask)
    (goto _label)))

(event `FinishTalk`
  (bind __abp_face_mask (`self. ABP Face Mask`))
  (bind _talkspeed (`/Game/CreativeTask/Characters/Face/ABP_Face.TalkSpeed` __abp_face_mask))
  (if (> _talkspeed 0.0) :!label _label_2
    (`KismetSystemLibrary.DelayUntilNextTick`)
    (set `/Game/CreativeTask/Characters/Face/ABP_Face.TalkSpeed` (`KismetMathLibrary.FInterpTo_Constant` _talkspeed 0.0 (`GameplayStatics.GetWorldDeltaSeconds`) 1.0) __abp_face_mask)
    (goto _label_2)
    (else
      (`KismetSystemLibrary.Delay` 1.0)
      (bind _returnvalue (`KismetMaterialLibrary.CreateDynamicMaterialInstance` "/Game/CreativeTask/Art/Materials/MI_Dissolve.MI_Dissolve"))
      (bind _output_get (set `self.DMI` _returnvalue))
      (`PrimitiveComponent.SetMaterial` (`self.SkeletalMesh`) 0 _output_get)
      (bind (_direction _dissolvetrack) (`Timeline|Timeline` :!via `PlayFromStart`)
        (:`Update`
          (`MaterialInstanceDynamic.SetScalarParameterValue` (`self.DMI`) "DissolveAmount" _dissolvetrack))
        (:`Finished`
          (`self.OnFinishTalk`))))))

(fn `UserConstructionScript`)